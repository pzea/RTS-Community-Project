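; Resource spawner for an RTS that scatters wood, gold or food actors, chosen by ResourceType, around itself when SpawnResources runs.
; If UsePCGrid is set, it briefly spawns an RTS controller to copy its GridSize, then destroys it.
; Each attempt box-traces grid-snapped random points within SpawnRadius, spawning only on Landscape hits, so the count can fall short of NumberOfResources.
; Each spawned resource gets a random size through SetResourceSize.
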(event Custom|SpawnResources
  (bind _returnvalue (Transformation|GetActorLocation))
  (bind _returnvalue_2 (Math|Random|RandomIntegerinRange 0 3))
  (bind _spawnradius (Variables|Default|GetSpawnRadius))
  (bind _returnvalue_3 (Class|NavigationSystem|GetRandomPointinRadius _returnvalue _spawnradius))
  (bind _returnvalue_4 (Math|Conversions|ToByte(Integer) _returnvalue_2))
  (bind (_x _y _z) (Math|Vector|BreakVector _returnvalue_3))
  (bind _returnvalue_5 (Utilities|Enum|ByteToEnumRTS_ENUM_ResourceSize _returnvalue_4))
  (Variables|Default|SetResourcesToSpawn (Variables|Default|GetNumberOfResources))
  (Utilities|FlowControl|Sequence
    (:then_0
      (if (Variables|Default|GetbUsePCGrid)
        (bind _returnvalue_6 (Game|SpawnActorfromClass "/Game/Blueprints/BP_RTS_Controller.BP_RTS_Controller_C" (Math|Transform|MakeTransform "0, 0, 0") true 0))
        (Variables|Default|SetGridSize (Variables|/Game/Blueprints/BP_RTS_Controller.BP_RTS_Controller_C|GetGridSize _returnvalue_6))
        (Actor|DestroyActor _returnvalue_6)))
    (:then_1
      (for _index (range 0 (Variables|Default|GetNumberOfResources))
        (bind _outhit (Collision|BoxTraceByChannel (+ (Math|Vector|MakeVector (Utilities|GridSnap _x (Variables|Default|GetGridSize)) (Utilities|GridSnap _y (Variables|Default|GetGridSize)) _z) "0,0.000000,200.000000") (Math|Vector|MakeVector (.X (Math|Vector|BreakVector (Math|Vector|MakeVector (Utilities|GridSnap _x (Variables|Default|GetGridSize)) (Utilities|GridSnap _y (Variables|Default|GetGridSize)) _z))) (.Y (Math|Vector|BreakVector (Math|Vector|MakeVector (Utilities|GridSnap _x (Variables|Default|GetGridSize)) (Utilities|GridSnap _y (Variables|Default|GetGridSize)) _z))) (.Z (Math|Vector|BreakVector (* (Math|Vector|MakeVector (Utilities|GridSnap _x (Variables|Default|GetGridSize)) (Utilities|GridSnap _y (Variables|Default|GetGridSize)) _z) 1e+04)))) (Math|Vector|MakeVector (Math|Conversions|ToFloat(Integer) (/ (Variables|Default|GetGridSize) 2)) (Math|Conversions|ToFloat(Integer) (/ (Variables|Default|GetGridSize) 2)) 1.0) (Class|KismetMathLibrary|MakeRot 0.0 0.0 0.0) "TraceTypeQuery1" false 0 (Variables|Default|GetDebugDraw)))
        (Utilities|Casting|CastToLandscape (.HitActor (Collision|BreakHitResult _outhit)))
        (switch Utilities|FlowControl|Switch|SwitchonRTS_ENUM_ResourceType (Variables|Default|GetResourceType)
          (:NewEnumerator0
            (bind _returnvalue_7 (Game|SpawnActorfromClass "/Game/Blueprints/Resources/BP_Wood.BP_Wood_C" (Math|Conversions|ToTransform(Vector) (.Location (Collision|BreakHitResult _outhit))) false 0))
            (Variables|/Game/Blueprints/BP_RTS_Resource_Master.BP_RTS_Resource_Master_C|SetResourceSize _returnvalue_7 _returnvalue_5)
            (Default|SetResourceSize _returnvalue_7 (Variables|/Game/Blueprints/BP_RTS_Resource_Master.BP_RTS_Resource_Master_C|GetResourceSize _returnvalue_7)))
          (:NewEnumerator1
            (bind _returnvalue_8 (Game|SpawnActorfromClass "/Game/Blueprints/Resources/BP_Gold.BP_Gold_C" (Math|Conversions|ToTransform(Vector) (.Location (Collision|BreakHitResult _outhit))) false 0))
            (Variables|/Game/Blueprints/BP_RTS_Resource_Master.BP_RTS_Resource_Master_C|SetResourceSize _returnvalue_8 _returnvalue_5)
            (Default|SetResourceSize _returnvalue_8 (Variables|/Game/Blueprints/BP_RTS_Resource_Master.BP_RTS_Resource_Master_C|GetResourceSize _returnvalue_8)))
          (:NewEnumerator2
            (bind _returnvalue_9 (Game|SpawnActorfromClass "/Game/Blueprints/Resources/BP_Food.BP_Food_C" (Math|Conversions|ToTransform(Vector) (.Location (Collision|BreakHitResult _outhit))) false 0))
            (Variables|/Game/Blueprints/BP_RTS_Resource_Master.BP_RTS_Resource_Master_C|SetResourceSize _returnvalue_9 _returnvalue_5)
            (Default|SetResourceSize _returnvalue_9 (Variables|/Game/Blueprints/BP_RTS_Resource_Master.BP_RTS_Resource_Master_C|GetResourceSize _returnvalue_9))))))))

(fn ConstructionScript)